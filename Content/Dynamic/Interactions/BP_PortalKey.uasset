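; BP_PortalKey is a collectible key actor tied to a portal, with custom-depth highlighting on focus.
; Interact triggers the portal's pickup message, hides the key, disables collision and reports it to My_gamestate.
; Respawn events show or hide the key, while a resettable DoOnce on overlap increments the player's KeysCollected.
; InterfaceInteract separately flips InteractToggle through InteractOnServer, but its OnRep point-light logic is disconnected.
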(event `respawningallkeys`
  (`KismetSystemLibrary.PrintString` "Hello")
  (`self.SetActorHiddenInGame` false)
  (`PrimitiveComponent.SetCollisionEnabled` (`self.BlocksCollision`) "QueryAndPhysics")
  (goto _label :!via `Reset`))

(event `self.ReceiveActorBeginOverlap`
  (params (OtherActor :type "Actor Object Reference"))
  (`/Engine/EditorBlueprintResources/StandardMacros.DoOnce` false :!label _label
    (:`Completed`
      (bind _asbp_player_character (cast `/Game/Dynamic/Blueprints/CHaracterMovement/BP_PlayerCharacter` OtherActor))
      (set `/Game/Dynamic/Blueprints/CHaracterMovement/BP_PlayerCharacter.KeysCollected` (+ (`/Game/Dynamic/Blueprints/CHaracterMovement/BP_PlayerCharacter.KeysCollected` _asbp_player_character) 1) _asbp_player_character))))

(event `Respawning keys`
  (`KismetSystemLibrary.PrintString` "wdadsdasdd")
  (`self.SetActorHiddenInGame` true)
  (`PrimitiveComponent.SetCollisionEnabled` (`self.BlocksCollision`) "NoCollision"))

(event `/Game/Dynamic/Interactions/BI_Interaction.Interact`
  (message `/Game/Dynamic/Interactions/BI_Portal.PickUpKey` (`self.Portal`))
  (`self.SetActorHiddenInGame` true)
  (`PrimitiveComponent.SetCollisionEnabled` (`self.BlocksCollision`) "NoCollision")
  (bind _asmy_gamestate (cast `/Game/Dynamic/Blueprints/checkpoints/My_gamestate` (`GameplayStatics.GetGameState`)))
  (`/Game/Dynamic/Blueprints/checkpoints/My_gamestate.Key colected` _asmy_gamestate self))

(event `self.Interface_ToggleFocus`
  (params (Focus :type Boolean))
  (`PrimitiveComponent.SetRenderCustomDepth` (`self.Cube`) Focus))

(event `self.InterfaceInteract`
  (`self.InteractOnServer`))

(event `InteractOnServer`
  (set `self.InteractToggle` (not (`self.InteractToggle`))))

(fn `GetInteractionWidgetRef`
  (returns (Ref :type "WidgetComponent Object Reference"))
  (return (`self.Widget`)))

(fn `OnRep_InteractToggle`
  ;[1 1 1] Visibility of Point light
)

(fn `UserConstructionScript`)