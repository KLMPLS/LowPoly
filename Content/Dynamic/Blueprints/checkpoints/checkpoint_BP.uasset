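; Checkpoint actor that saves a respawn point the first time any actor overlaps its Box.
; It loads the "checksave" Save_Game_OBJ, or creates one if none exists, then writes its own location and the overlapping actor's forward vector as player location and rotation.
; After saving to the slot, it calls GameIsSaving on My_gamestate.
; A DoOnce limits it to one save, with no filter on the overlapping actor.
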(event `self.Box.OnComponentBeginOverlap`
  (params (OverlappedComponent :type "PrimitiveComponent Object Reference") (OtherActor :type "Actor Object Reference") (OtherComp :type "PrimitiveComponent Object Reference") (OtherBodyIndex :type Integer) (bFromSweep :type Boolean) (SweepResult :type "HitResult Structure (by ref)"))
  (bind _returnvalue (`self.K2_GetActorLocation`))
  (`/Engine/EditorBlueprintResources/StandardMacros.DoOnce` false
    (:`Completed`
      (bind _returnvalue_2 (`GameplayStatics.DoesSaveGameExist` "checksave"))
      (if _returnvalue_2
        (bind _returnvalue_3 (`GameplayStatics.LoadGameFromSlot` "checksave"))
        (bind _assave_game_obj (cast `/Game/Dynamic/Blueprints/checkpoints/Save_Game_OBJ` _returnvalue_3))
        (set `/Game/Dynamic/Blueprints/checkpoints/Save_Game_OBJ.PlayerLoc` _returnvalue _assave_game_obj)
        (set `/Game/Dynamic/Blueprints/checkpoints/Save_Game_OBJ.PlayerRot` (`KismetMathLibrary.Conv_RotatorToVector` (`self.K2_GetActorRotation` OtherActor)) _assave_game_obj)
        (`GameplayStatics.SaveGameToSlot` _assave_game_obj "checksave")
        (else
          (bind _returnvalue_4 (`GameplayStatics.CreateSaveGameObject` "/Game/Dynamic/Blueprints/checkpoints/Save_Game_OBJ.Save_Game_OBJ_C"))
          (set `/Game/Dynamic/Blueprints/checkpoints/Save_Game_OBJ.PlayerLoc` _returnvalue _returnvalue_4)
          (set `/Game/Dynamic/Blueprints/checkpoints/Save_Game_OBJ.PlayerRot` (`KismetMathLibrary.Conv_RotatorToVector` (`self.K2_GetActorRotation` OtherActor)) _returnvalue_4)
          (`GameplayStatics.SaveGameToSlot` _returnvalue_4 "checksave")))
      (bind _asmy_gamestate (cast `/Game/Dynamic/Blueprints/checkpoints/My_gamestate` (`GameplayStatics.GetGameState`)))
      (`/Game/Dynamic/Blueprints/checkpoints/My_gamestate.Game_is_saving` _asmy_gamestate))))

(fn `UserConstructionScript`)