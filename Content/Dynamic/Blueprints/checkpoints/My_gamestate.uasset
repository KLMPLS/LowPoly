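; Game state Blueprint that tracks collected keys and persists them for checkpoints through the "checksave" save slot.
; Keycolected records each key reference and increments a count, which Game_is_saving writes into the existing Save_Game_OBJ.
; Keysrefresh calls Respawningallkeys on tracked keys, restores the saved array and player's KeysCollected, then calls RespawningKeys on saved keys.
; The refresh leaves its own Ammountcollectedkeys counter unrestored.
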(event `Keysrefresh`
  (`|ExecutionSequence`
    (:`then_0`
      (for _array_element (`self.whichkeyscolected`)
        (`/Game/Dynamic/Interactions/BP_PortalKey.respawningallkeys` _array_element)))
    (:`then_1`
      (bind _returnvalue (`GameplayStatics.LoadGameFromSlot` "checksave"))
      (bind _assave_game_obj (cast `/Game/Dynamic/Blueprints/checkpoints/Save_Game_OBJ` _returnvalue))
      (bind _arrayofkeyscolected (`/Game/Dynamic/Blueprints/checkpoints/Save_Game_OBJ.Arrayofkeyscolected` _assave_game_obj))
      (set `self.whichkeyscolected` _arrayofkeyscolected)
      (bind _asbp_player_character (cast `/Game/Dynamic/Blueprints/CHaracterMovement/BP_PlayerCharacter` (`GameplayStatics.GetPlayerCharacter` 0))
        (:`then`
          (set `/Game/Dynamic/Blueprints/CHaracterMovement/BP_PlayerCharacter.KeysCollected` (`KismetMathLibrary.Conv_IntToByte` (`/Game/Dynamic/Blueprints/checkpoints/Save_Game_OBJ.Ammountofkeyscollected` _assave_game_obj)) _asbp_player_character)
          (for _array_element_2 _arrayofkeyscolected
            (`/Game/Dynamic/Interactions/BP_PortalKey.Respawning keys` _array_element_2)))
        (:`CastFailed`
          (`KismetSystemLibrary.PrintString` "Heladhgfhofhiuhfoidsfiugduofgkdjfgahbdfhjagfiuahdiufhdsiflo"))))))

(event `Game_is_saving`
  (bind _returnvalue (`GameplayStatics.LoadGameFromSlot` "checksave"))
  (bind _assave_game_obj (cast `/Game/Dynamic/Blueprints/checkpoints/Save_Game_OBJ` _returnvalue))
  (set `/Game/Dynamic/Blueprints/checkpoints/Save_Game_OBJ.Arrayofkeyscolected` (`self.whichkeyscolected`) _assave_game_obj)
  (bind _output_get (set `/Game/Dynamic/Blueprints/checkpoints/Save_Game_OBJ.Ammountofkeyscollected` (stale `Key colected` _output_get) _assave_game_obj))
  (`KismetSystemLibrary.PrintString` (`KismetStringLibrary.Conv_IntToString` _output_get))
  (`GameplayStatics.SaveGameToSlot` _assave_game_obj "checksave"))

(event `Key colected`
  (params (referenceNewParam :type "/Game/Dynamic/Interactions/BP_PortalKey Object Reference"))
  (`KismetArrayLibrary.Array_Add` (`self.whichkeyscolected`) referenceNewParam)
  (bind _output_get (set `self.Ammountcollectedkeys` (+ (`self.Ammountcollectedkeys`) 1))))

(fn `UserConstructionScript`)